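; BP_AI_Bot is an AI controller that runs guard behavior for NPC bots and tracks perceived targets.
; On BeginPlay it initializes the PatrolData blackboard and starts the Guard_Behaviour tree.
; Perception updates write sensed actors lacking the "Enemy" tag to the Enemy blackboard key.
; When such an actor's stimulus is lost, it clears that key and the controller's focus.
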(event OnTargetPerceptionUpdated(AIPerception)
  (params (Actor :type Actor%20Object%20Reference) (Stimulus :type AI%20Stimulus%20Structure))
  (bind _returnvalue (Utilities|String|StringToName "Enemy"))
  (bind _blackboardcomp (Variables|Default|GetBlackboardComp))
  (if (not (Actor|ActorHasTag Actor "Enemy"))
    (if (.bSuccessfullySensed (Utilities|Struct|BreakAIStimulus Stimulus))
      (AI|Components|Blackboard|SetValueasObject _blackboardcomp _returnvalue Actor)
      (else
        (AI|Components|Blackboard|ClearValue _blackboardcomp _returnvalue)
        (AI|ClearFocus)))))

(event EventBeginPlay
  (bind _blackboardcomponent (Class|AIController|UseBlackboard "/Game/NPC/AI/PatrolData.PatrolData"))
  (Variables|Default|SetBlackboardComp _blackboardcomponent)
  (AI|RunBehaviorTree "/Game/NPC/AI/Guard_Behaviour.Guard_Behaviour"))

(fn ConstructionScript)