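; Game mode for an endless terrain level that spawns level blocks chained end to end and tracks a score.
; On BeginPlay it populates a nav mesh and spawns four starting blocks, each at the attach point of the previous one.
; Each block receives the shared NavMeshBounds pool, then randomly places props, rocks and patrolling AI pawns.
; TilePassed increments the score.
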(event EventBeginPlay
  (Class|InfiniteTerrainGameMode|PopulateNavMesh)
  (for _index (range 0 3)
    (CallFunction|SpawnBlock)))

(fn ConstructionScript)

(fn SpawnBlock
  (bind _returnvalue (Game|SpawnActorfromClass "/Game/Terrain/BP_LevelBlock.BP_LevelBlock_C" (Variables|Default|GetNext%20Tile%20Spawn%20Transform) "Undefined" 0 0))
  (Class|Tile|SetPool _returnvalue (Variables|Default|GetNavMeshBoundsPool))
  (bind _newparam (Default|GetAttachLocation _returnvalue))
  (Variables|Default|SetNext%20Tile%20Spawn%20Transform _newparam)
  (Class|Tile|PlaceActors _returnvalue "/Game/Terrain/Props/BP_Container.BP_Container_C" 2 5 5e+02 1.0 1.0)
  (Class|Tile|PlaceActors _returnvalue "/Game/Terrain/Props/BP_Canister.BP_Canister_C" 1 6 4e+01 1.0 1.0)
  (Class|Tile|PlaceActors _returnvalue "/Game/Terrain/Props/BP_Box.BP_Box_C" 1 6 115.0 1.0 1.0)
  (Class|Tile|PlaceActors _returnvalue "/Game/Terrain/Props/BP_Rock1.BP_Rock1_C" 1 5 2.5e+02 1.0 3.0)
  (Class|Tile|PlaceActors _returnvalue "/Game/Terrain/Props/BP_Rock2.BP_Rock2_C" 1 5 3e+02 1.0 3.0)
  (Class|Tile|PlaceActors _returnvalue "/Game/Terrain/Props/BP_Rock3.BP_Rock3_C" 1 5 1.5e+02 1.0 3.0)
  (Class|Tile|PlaceActors _returnvalue "/Game/Terrain/Props/BP_Sandbags.BP_Sandbags_C" 0 3 2.5e+02 1.0 1.0)
  (Class|Tile|PlaceAIPawns _returnvalue "/Game/Character/Behaviour/BP_Patrolling_Character.BP_Patrolling_Character_C" 2 4 1.5e+02))

(fn TilePassed
  (Math|Integer|IncrementInt (Variables|Default|GetScore)))